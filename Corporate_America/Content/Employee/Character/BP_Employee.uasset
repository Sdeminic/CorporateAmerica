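; BP_Employee is the employee character Blueprint, implementing a networked variable-height jump.
; Jump input runs the jump logic locally and also calls server jump functions, whose bound events on BeginPlay run the same logic.
; A grounded jump briefly lowers gravity scale, then raises it after a short delay or on release for a snappier, heavier fall.
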(event Custom|ServerJump_Event
  (bind _charactermovement (Variables|Character|GetCharacterMovement))
  (if (not (AI|Components|NavMovement|IsFalling _charactermovement))
    (Variables|/Script/Engine.CharacterMovementComponent|SetGravityScale _charactermovement 1.0)
    (Character|Jump)
    (Utilities|FlowControl|Delay 0.2)
    (Variables|/Script/Engine.CharacterMovementComponent|SetGravityScale _charactermovement 4.0)))

(event Custom|ServerEndJump_Event
  (Variables|/Script/Engine.CharacterMovementComponent|SetGravityScale (Variables|Character|GetCharacterMovement) 4.0)
  (Character|StopJumping))

(event EventBeginPlay
  (EventDispatchers|BindEventtoServerJump (delegate Custom|ServerJump_Event))
  (EventDispatchers|BindEventtoServerEndJump (delegate Custom|ServerEndJump_Event)))

(event Input|ActionEvents|InputActionJump
  (params (Key :type Key%20Structure))
  (bind _charactermovement (Variables|Character|GetCharacterMovement))
  (:Pressed
    (Default|CallServerJump)
    (if (not (AI|Components|NavMovement|IsFalling _charactermovement))
      (Variables|/Script/Engine.CharacterMovementComponent|SetGravityScale _charactermovement 1.0)
      (Character|Jump)
      (Utilities|FlowControl|Delay 0.2)
      (Variables|/Script/Engine.CharacterMovementComponent|SetGravityScale _charactermovement 4.0)))
  (:Released
    (Default|CallServerEndJump)
    (Variables|/Script/Engine.CharacterMovementComponent|SetGravityScale (Variables|Character|GetCharacterMovement) 4.0)
    (Character|StopJumping)))

(fn ConstructionScript)